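; BP_Mothman is a physics-driven moth actor that homes in on nearby lights and damages destructibles it hits.
; Each tick it gets the nearest light in range, accelerates toward it under a slowly rising speed cap with corrective damping, and turns its child actor.
; Hits reflect its direction and slash speed; the disorient timer check is unwired, so targeting resumes next tick.
; A debug sphere shows range and lock state.
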(event EventBeginPlay
  (Variables|Default|SetCurrentDirection (Math|Random|RandomUnitVector))
  (Rendering|SetVisibility (Variables|Default|GetCollider) false false))

(event Collision|EventActorBeginOverlap
  (params (OtherActor :type Actor%20Object%20Reference)))

(event EventTick
  (params (DeltaSeconds :type Float%20%28single-precision%29))
  (CallFunction|UpdateTarget)
  (CallFunction|UpdateVelocity DeltaSeconds)
  (Rendering|Debug|DrawDebugSphere (Transformation|GetActorLocation) (Variables|Default|GetLightViewRange) 12 (Variables|Default|GetTargetDebugColour) 0.0)
  (Variables|Default|SetMaxSpeed (+ (* DeltaSeconds 0.1) (Variables|Default|GetMaxSpeed)))
  (bind _returnvalue (Physics|GetPhysicsLinearVelocity (Variables|Default|GetCollider) "None"))
  (Transformation|SetWorldRotation (Variables|Default|GetChildActor) (Math|Rotator|FindLookatRotation (Math|Vector|MakeVector 0.0 0.0 0.0) _returnvalue) false false))

(event Collision|EventHit
  (params (MyComp :type Primitive%20Component%20Object%20Reference) (Other :type Actor%20Object%20Reference) (OtherComp :type Primitive%20Component%20Object%20Reference) (bSelfMoved :type Boolean) (HitLocation :type Vector :default "0, 0, 0") (HitNormal :type Vector :default "0, 0, 0") (NormalImpulse :type Vector :default "0, 0, 0") (Hit :type Hit%20Result%20Structure%20%28by%20ref%29))
  (CallFunction|Disorient)
  (Variables|Default|SetCurrentSpeed (* (Variables|Default|GetCurrentSpeed) 0.1))
  (Variables|Default|SetCurrentDirection (- (Variables|Default|GetCurrentDirection) (* HitNormal (Math|Vector|DotProduct HitNormal (Variables|Default|GetCurrentDirection)) 2.0)))
  (bind _asbp_destructible_base (Utilities|Casting|CastToBP_Destructible_Base Other))
  (Default|TakeDamage _asbp_destructible_base (Variables|Default|GetDamage)))

(fn ConstructionScript)

(fn UpdateVelocity
  (params (dt :type Float%20%28double-precision%29))
  (bind _maxspeed (Variables|Default|GetMaxSpeed))
  (if (<= (+ (* dt (Variables|Default|GetAcceleration)) (Variables|Default|GetCurrentSpeed)) _maxspeed)
    (Variables|Default|SetCurrentSpeed (+ (* dt (Variables|Default|GetAcceleration)) (Variables|Default|GetCurrentSpeed)))
    (else
      (Variables|Default|SetCurrentSpeed _maxspeed)))
  (bind _output_get (Variables|Default|SetCurrentVeclocity (* (Variables|Default|GetCurrentSpeed) (Variables|Default|GetCurrentDirection))))
  (Physics|AddForce (Variables|Default|GetCollider) _output_get "None" true)
  (if (Variables|Default|GetHasTarget)
    (bind _returnvalue (Physics|GetPhysicsLinearVelocity (Variables|Default|GetCollider) "None"))
    (Physics|AddForce (Variables|Default|GetCollider) (* (/ (* _returnvalue -1.0) 2.0) (/ (+ (* (Math|Vector|DotProduct (Variables|Default|GetCurrentDirection) _returnvalue) -1.0) 1.0) 2.0)) "None" false)))

(fn UpdateTarget
  (bind (_light _foundlight) (Default|GetNearestTarget (Variables|Default|Getgm) (Transformation|GetActorLocation) (Variables|Default|GetLightViewRange)))
  (bind _output_get (Variables|Default|SetHasTarget _foundlight))
  (if _output_get
    (bind _location (Default|GetGlobeTransform _light))
    (Variables|Default|SetTargetPos _location)
    (Variables|Default|SetCurrentDirection (Math|Vector|GetUnitDirection(Vector) (Transformation|GetActorLocation) (Variables|Default|GetTargetPos)))
    (Variables|Default|SetTargetDebugColour "(R=0.000000,G=1.000000,B=0.000000,A=0.500000)")
    (else
      (Variables|Default|SetTargetDebugColour "(R=1.000000,G=0.000000,B=0.000000,A=0.500000)")))
  (return (Variables|Default|GetHasTarget)))

(fn UpdateDisorient
  (params (dt :type Float%20%28double-precision%29))
  (if (Variables|Default|GetIsDisoriented)
    (bind _output_get (Variables|Default|SetDisorientedTimer (- (Variables|Default|GetDisorientedTimer) dt)))
    (Variables|Default|SetIsDisoriented (> _output_get 0.0)))
  (return (Variables|Default|GetIsDisoriented)))

(fn Disorient
  (Variables|Default|SetIsDisoriented true)
  (Variables|Default|SetDisorientedTimer (Variables|Default|GetDisorientedDelay))
  (Variables|Default|SetHasTarget false)
  (Variables|Default|SetTargetDebugColour "(R=1.000000,G=0.000000,B=0.000000,A=0.500000)"))