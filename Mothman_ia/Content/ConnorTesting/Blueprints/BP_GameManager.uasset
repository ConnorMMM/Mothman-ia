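; BP_GameManager is a manager actor that tracks the level's lamps and answers nearest-light queries.
; On BeginPlay it caches every SD_Lamp_Base actor in an AllLights array.
; GetNearestLightInRange scans that cache for enabled lamps, measures distance to each globe transform, and returns the closest location within range, or the input position if none qualifies.
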(event EventBeginPlay
  (bind _outactors (Actor|GetAllActorsOfClass "/Game/Blueprints/Devices/Base/SD_Lamp_Base.SD_Lamp_Base_C"))
  (Variables|Default|SetAll_Lights _outactors))

(event Collision|EventActorBeginOverlap
  (params (OtherActor :type Actor%20Object%20Reference)))

(event EventTick
  (params (DeltaSeconds :type Float%20%28single-precision%29)))

(fn ConstructionScript)

(fn GetNearestLightinRange
  (params (Position :type Vector) (Range :type Float%20%28double-precision%29))
  (Variables|Default|SetFoundLight false)
  (Variables|Default|SetClosestLightDis Range)
  (for _array_element (Variables|Default|GetAll_Lights)
    (bind _device_info (Default|GetDeviceInfo _array_element))
    (if (.enabled _device_info)
      (bind _location (Default|GetGlobeTransform _array_element))
      (if (<= (Math|Vector|Distance(Vector) _location Position) (Variables|Default|GetClosestLightDis))
        (Variables|Default|SetFoundLight true)
        (Variables|Default|SetClosestLightDis (Math|Vector|Distance(Vector) _location Position))
        (Variables|Default|SetClosestLightPos _location))))
  (if (Variables|Default|GetFoundLight)
    (return (Variables|Default|GetClosestLightPos))
    (else
      (return Position))))