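; BP_Mothman is a physics-driven moth creature that flies in a random direction until drawn to a nearby light.
; Tick asks Gm for the nearest light in range, treating its own location as none found, and steers toward any light with a large boost.
; UpdateVelocity applies acceleration force capped by MaxSpeed, which creeps up while no light is found.
; Hits reflect the heading off the surface normal.
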(event EventBeginPlay
  (Variables|Default|SetCurrentDirection (Math|Random|RandomUnitVector)))

(event Collision|EventActorBeginOverlap
  (params (OtherActor :type Actor%20Object%20Reference)))

(event EventTick
  (params (DeltaSeconds :type Float%20%28single-precision%29))
  (bind _returnvalue (Transformation|GetActorLocation))
  (bind _light_pos (Default|GetNearestLightinRange (Variables|Default|Getgm) _returnvalue (Variables|Default|GetLightViewRange)))
  (if (Utilities|Operators|EqualEqual _light_pos _returnvalue 0.0)
    (CallFunction|UpdateVelocity (Variables|Default|GetCurrentDirection) DeltaSeconds 0.0)
    (Variables|Default|SetMaxSpeed (+ (Variables|Default|GetMaxSpeed) (* DeltaSeconds 0.1)))
    (Transformation|SetRelativeScale3D (Variables|Default|GetSphere) (Math|Conversions|ToVector(Float) (* (Variables|Default|GetLightViewRange) 0.04)))
    (Transformation|SetRelativeLocation (Variables|Default|GetSphere1) (Math|Conversions|ToVector(Float) (Variables|Default|GetLightViewRange)) false false)
    (else
      (Variables|Default|SetCurrentDirection (Math|Vector|GetUnitDirection(Vector) _returnvalue _light_pos))
      (CallFunction|UpdateVelocity (Math|Vector|GetUnitDirection(Vector) _returnvalue _light_pos) DeltaSeconds 5e+05))))

(event Collision|EventHit
  (params (MyComp :type Primitive%20Component%20Object%20Reference) (Other :type Actor%20Object%20Reference) (OtherComp :type Primitive%20Component%20Object%20Reference) (bSelfMoved :type Boolean) (HitLocation :type Vector :default "0, 0, 0") (HitNormal :type Vector :default "0, 0, 0") (NormalImpulse :type Vector :default "0, 0, 0") (Hit :type Hit%20Result%20Structure%20%28by%20ref%29))
  (Variables|Default|SetCurrentSpeed (* (Variables|Default|GetCurrentSpeed) 0.8))
  (Variables|Default|SetCurrentDirection (- (Variables|Default|GetCurrentDirection) (* HitNormal (Math|Vector|DotProduct HitNormal (Variables|Default|GetCurrentDirection)) 2.0))))

(fn ConstructionScript)

(fn UpdateVelocity
  (params (Direction :type Vector) (dt :type Float%20%28double-precision%29) (MovingTowardsLight :type Float%20%28double-precision%29))
  (bind _acceleration (Variables|Default|GetAcceleration))
  (bind _maxspeed (Variables|Default|GetMaxSpeed))
  (bind _returnvalue (+ MovingTowardsLight _acceleration))
  (bind _returnvalue_2 (* dt _returnvalue))
  (bind _returnvalue_3 (* Direction _returnvalue_2))
  (bind _returnvalue_4 (Math|Vector|VectorLength _returnvalue_3))
  (if (> _returnvalue_4 _maxspeed)
    (Physics|AddForce (Variables|Default|GetCollider) (* _returnvalue_3 (/ _maxspeed _returnvalue_4)) "None" true)
    (else
      (Physics|AddForce (Variables|Default|GetCollider) _returnvalue_3 "None" true))))