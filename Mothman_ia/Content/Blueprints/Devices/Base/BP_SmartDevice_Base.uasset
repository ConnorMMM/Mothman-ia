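; BP_SmartDevice_Base is a base Blueprint for smart devices that can be switched on and off.
; ToggleDevice writes the enabled flag in DeviceInfo and fires OnDeviceStateChange, while Interact inverts the current state through it.
; EnableDevice and DisableDevice both pass false to ToggleDevice, so both switch the device off.
; Getters expose DeviceInfo and the Interactable flag through IsInteractive, while the separate IsInteractable always returns false.
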(event EventBeginPlay)

(event Collision|EventActorBeginOverlap
  (params (OtherActor :type Actor%20Object%20Reference)))

(event EventTick
  (params (DeltaSeconds :type Float%20%28single-precision%29)))

(event Custom|Enable%20Device
  (CallFunction|ToggleDevice false))

(event Custom|Disable%20Device
  (CallFunction|ToggleDevice false))

(event Custom|Toggle%20Device
  (params (Enable :type Boolean))
  ;[1 1 1] Sets the Base state of the device and calls the state changed event
  (|SetBy-RefVar (.enabled (Variables|Device|GetDevice%20Info)) Enable)
  (Default|CallOnDeviceStateChange Enable))

(event EventInteract
  (CallFunction|ToggleDevice (not (.enabled (Variables|Device|GetDevice%20Info)))))

(fn ConstructionScript)

(fn IsInteractive
  (return (Variables|Device|GetInteractable)))

(fn GetDeviceInfo
  (return (Variables|Device|GetDevice%20Info)))

(fn IsInteractable
  (return false))